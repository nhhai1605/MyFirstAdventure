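; AI controller for the pig enemy that runs the shared enemy behavior tree and blackboard, targeting player 0's main character from BeginPlay.
; On possession it binds to the pig's can-act state changes and mirrors them into the blackboard.
; SetFocusDirection offsets the focal point by the X component of the look-at direction to a valid target while the pig can act, otherwise keeping it straight ahead.
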(event `self.ReceivePossess`
  (params (PossessedPawn :type "Pawn Object Reference"))
  (bind _asbp_pig (cast `/Game/Blueprints/Characters/Pig/BP_Pig` PossessedPawn))
  (bind _output_get (set `self.Pig` _asbp_pig))
  (add `/Game/Blueprints/Characters/BP_BaseCharacter.CanActStateChanged` _output_get (delegate `OnCanActStateChanged`)))

(event `OnCanActStateChanged`
  (params (CanAct :type Boolean))
  (`BlackboardComponent.SetValueAsBool` (`self.Blackboard`) (`self.CanActKey`) CanAct))

(event `self.ReceiveBeginPlay`
  (`self.UseBlackboard` "/Game/Blueprints/AI/BB_Enemy.BB_Enemy")
  (`self.RunBehaviorTree` "/Game/Blueprints/AI/BT_Enemy.BT_Enemy")
  (bind _asbp_main_character (cast `/Game/Blueprints/Characters/MainCharacter/BP_MainCharacter` (`GameplayStatics.GetPlayerPawn` 0)))
  (`self.SetAttackTarget` _asbp_main_character))

(fn `SetAttackTarget`
  (params (AttackTarget :type "/Game/Blueprints/Characters/BP_BaseCharacter Object Reference"))
  (`BlackboardComponent.SetValueAsObject` (`self.Blackboard`) (`self.AttackTargetKey`) AttackTarget)
  (set `self.AttackTarget` AttackTarget))

(fn `SetFocusDirection`
  (bind _pig (`self.Pig`))
  (bind _returnvalue_x (`KismetMathLibrary.BreakVector` (`KismetMathLibrary.GetForwardVector` (`KismetMathLibrary.FindLookAtRotation` (`self.K2_GetActorLocation` (`self.Pig`)) (`self.K2_GetActorLocation` (`self.AttackTarget`))))))
  (`/Engine/EditorBlueprintResources/StandardMacros.IsValid` (`self.AttackTarget`)
    (:`Is Valid`
      (bind _canact (`/Game/Blueprints/Characters/BP_BaseCharacter.CanAct` (`self.Pig`)))
      (if _canact
        (`self.K2_SetFocalPoint` (+ _returnvalue_x (`self.K2_GetActorLocation` (`self.Pig`))))
        (else
          (`self.K2_SetFocalPoint` (+ (`self.K2_GetActorLocation` _pig) (`self.GetActorForwardVector` _pig)) :!label _label))))
    (:`Is Not Valid`
      (goto _label))))

(fn `UserConstructionScript`)