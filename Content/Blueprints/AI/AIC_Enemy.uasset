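; AI controller for enemy characters that runs the BT_Enemy behavior tree on the BB_Enemy blackboard.
; On possess it binds to the BP_BaseCharacter's can-act event to mirror that state into the blackboard; SetAttackTarget stores the target there and locally.
; Each tick it sets the focal point toward the target along world X only, or straight ahead when there is no target or the character cannot act.
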(event `self.ReceivePossess`
  (params (PossessedPawn :type "Pawn Object Reference"))
  (bind _asbp_base_character (cast `/Game/Blueprints/Characters/BP_BaseCharacter` PossessedPawn))
  (bind _output_get (set `self.CurrentCharacter` _asbp_base_character))
  (add `/Game/Blueprints/Characters/BP_BaseCharacter.CanActStateChanged` _output_get (delegate `OnCanActStateChanged`)))

(event `OnCanActStateChanged`
  (params (CanAct :type Boolean))
  (`BlackboardComponent.SetValueAsBool` (`self.Blackboard`) (`self.CanActKey`) CanAct))

(event `self.ReceiveBeginPlay`
  (`self.UseBlackboard` "/Game/Blueprints/AI/BB_Enemy.BB_Enemy")
  (`self.RunBehaviorTree` "/Game/Blueprints/AI/BT_Enemy.BT_Enemy"))

(event `self.ReceiveTick`
  (params (DeltaSeconds :type "Float (single-precision)"))
  (`self.SetFocusDirection`))

(fn `SetAttackTarget`
  (params (AttackTarget :type "/Game/Blueprints/Characters/BP_BaseCharacter Object Reference"))
  (`BlackboardComponent.SetValueAsObject` (`self.Blackboard`) (`self.AttackTargetKey`) AttackTarget)
  (set `self.AttackTarget` AttackTarget))

(fn `SetFocusDirection`
  (bind _currentcharacter (`self.CurrentCharacter`))
  (bind _returnvalue_x (`KismetMathLibrary.BreakVector` (`KismetMathLibrary.GetForwardVector` (`KismetMathLibrary.FindLookAtRotation` (`self.K2_GetActorLocation` (`self.CurrentCharacter`)) (`self.K2_GetActorLocation` (`self.AttackTarget`))))))
  (`/Engine/EditorBlueprintResources/StandardMacros.IsValid` (`self.AttackTarget`)
    (:`Is Valid`
      (bind _canact (`/Game/Blueprints/Characters/BP_BaseCharacter.CanAct` (`self.CurrentCharacter`)))
      (if _canact
        (`self.K2_SetFocalPoint` (+ (`self.K2_GetActorLocation` (`self.CurrentCharacter`)) (`KismetMathLibrary.MakeVector` _returnvalue_x)))
        (else
          (`self.K2_SetFocalPoint` (+ (`self.K2_GetActorLocation` _currentcharacter) (`self.GetActorForwardVector` _currentcharacter)) :!label _label))))
    (:`Is Not Valid`
      (goto _label))))

(fn `UserConstructionScript`)