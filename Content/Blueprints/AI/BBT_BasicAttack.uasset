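; Behavior tree task that makes an AI-controlled BP_BaseCharacter perform its basic attack.
; If the character is not already attacking, it plays the character's attack sequence as an animation override in BasicAttackSlot and sets IsBasicAttacking.
; On completion or cancellation it waits the character's attack delay, then finishes with success or failure respectively and clears the flag.
; When the cast fails or an attack is already running, the task never calls FinishExecute.
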(event `self.ReceiveExecuteAI`
  (params (OwnerController :type "AIController Object Reference") (ControlledPawn :type "Pawn Object Reference"))
  (bind _asbp_base_character (cast `/Game/Blueprints/Characters/BP_BaseCharacter` ControlledPawn))
  (if (not (`/Game/Blueprints/Characters/BP_BaseCharacter.IsBasicAttacking` _asbp_base_character))
    (`PaperZDPlaySlotOverrideAction.PlayAnimationOverrideWithCallbacks` (`PaperZDCharacter.AnimInstance` _asbp_base_character) (`/Game/Blueprints/Characters/BP_BaseCharacter.BasicAttackAnimSequence` _asbp_base_character) "BasicAttackSlot"
      (:`then`
        (set `/Game/Blueprints/Characters/BP_BaseCharacter.IsBasicAttacking` true _asbp_base_character))
      (:`OnCompleted`
        (bind _attackdelayduration (`/Game/Blueprints/Characters/BP_BaseCharacter.AttackDelayDuration` _asbp_base_character))
        (`KismetSystemLibrary.RetriggerableDelay` _attackdelayduration)
        (`self.FinishExecute` true)
        (set `/Game/Blueprints/Characters/BP_BaseCharacter.IsBasicAttacking` false _asbp_base_character :!label _label))
      (:`OnCancelled`
        (`KismetSystemLibrary.RetriggerableDelay` _attackdelayduration)
        (`self.FinishExecute` false)
        (goto _label)))))