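; Behavior tree task that makes an AI enemy chase its attack target along the world X axis.
; Each tick it caches the AIC_Enemy controller and BP_BaseCharacter pawn, then finishes successfully once the target is within the acceptance radius.
; Otherwise ChaseTarget applies movement input toward the target's side, using direct input rather than pathfinding.
; Movement input is withheld when the character's wall or ledge check is true, leaving the task running.
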(event `self.ReceiveTickAI`
  (params (OwnerController :type "AIController Object Reference") (ControlledPawn :type "Pawn Object Reference") (DeltaSeconds :type "Float (single-precision)"))
  (bind _asaic_enemy (cast `/Game/Blueprints/AI/AIC_Enemy` OwnerController))
  (set `self.AIC` _asaic_enemy)
  (bind _asbp_base_character (cast `/Game/Blueprints/Characters/BP_BaseCharacter` ControlledPawn))
  (set `self.CurrentCharacter` _asbp_base_character)
  (if (<= (`Actor.GetDistanceTo` (`/Game/Blueprints/AI/AIC_Enemy.AttackTarget` (`self.AIC`)) (`self.CurrentCharacter`)) (`self.AcceptanceRadius`))
    (`self.FinishExecute` true)
    (else
      (`self.ChaseTarget`))))

(fn `ChaseTarget`
  (bind _currentcharacter (`self.CurrentCharacter`))
  (bind _returnvalue_x (`KismetMathLibrary.BreakVector` (`Actor.K2_GetActorLocation` (`self.CurrentCharacter`))))
  (bind _returnvalue_x_2 (`KismetMathLibrary.BreakVector` (`Actor.K2_GetActorLocation` (`/Game/Blueprints/AI/AIC_Enemy.AttackTarget` (`self.AIC`)))))
  (bind _seewall (`/Game/Blueprints/Characters/BP_BaseCharacter.CheckWall` _currentcharacter true))
  (bind _seeledge (`/Game/Blueprints/Characters/BP_BaseCharacter.CheckLedge` _currentcharacter true))
  (if (not (or _seeledge _seewall))
    (`Pawn.AddMovementInput` _currentcharacter (1.0 0.0 0.0) (`KismetMathLibrary.SelectFloat` 1.0 -1.0 (> _returnvalue_x_2 _returnvalue_x)) false)))